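; Traffic game controller that tracks play time and score, then ends the session at a time limit.
; BeginPlay loads the last used player profile through the MainSave slot.
; AddToScore accumulates arrived cars and pedestrians, accidents and road rage, then recalculates a score that rewards arrivals and penalizes incidents.
; Tick counts time and, once at the limit, passes stats to the profile, shows the GameOver widget and pauses.
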(event `self.ReceiveBeginPlay`
  ;[1 1 1] Get Current Profile
  (bind _returnvalue (`GameplayStatics.LoadGameFromSlot` "MainSave"))
  (bind _asmain_save (cast `/Game/Blueprints/SaveBlueprint/MainSave` _returnvalue))
  (bind _returnvalue_2 (`GameplayStatics.LoadGameFromSlot` (`/Game/Blueprints/SaveBlueprint/MainSave.LastUsedProfile` _asmain_save)))
  (bind _asplayer_profile (cast `/Game/Blueprints/SaveBlueprint/PlayerProfile` _returnvalue_2))
  (set `self.Current` _asplayer_profile))

(event `self.ReceiveTick`
  (params (DeltaSeconds :type "Float (single-precision)"))
  ;[1 1 1] Increase time
  (bind _output_get (set `self.Time` (+ DeltaSeconds (`self.Time`))))
  ;[1 1 1] Check if the time is over the time limit
  (if (>= _output_get (`self.TimeLimit`))
    ;[1 1 1] GameOver screen
    (`/Engine/EditorBlueprintResources/StandardMacros.DoOnce` false
      (:`Completed`
        (`self.UpdateCurrentSave`)
        (`/Engine/EditorBlueprintResources/StandardMacros.IsValid` (`self.GameOverScreenRef`)
          (:`Is Valid`
            _)
          (:`Is Not Valid`
            (bind _returnvalue (`|CreateWidget` "/Game/Blueprints/UserInterface/GameOverScreen.GameOverScreen_C"))
            (bind _output_get_2 (set `self.GameOverScreenRef` _returnvalue))))
        (`UserWidget.AddToViewport` _output_get_2 0)
        (`GameplayStatics.SetGamePaused` true)))))

(fn `Add to score`
  (params (CarsReachedDest :type Integer) (PedestriansReachingDest :type Integer) (Acidents :type Integer) (RoadRage :type Integer))
  ;[1 1 1] Get all imputs and add then to their respective varibles, they are 0 by defualt, so they will not increase unless set to somthing higher or lower then 1
  (set `self.CarsReachedDest` (+ CarsReachedDest (`self.CarsReachedDest`)))
  (set `self.PedsReachDest` (+ PedestriansReachingDest (`self.PedsReachDest`)))
  (set `self.Acidents` (+ Acidents (`self.Acidents`)))
  (set `self.RoadRage` (+ RoadRage (`self.RoadRage`)))
  (`self.Calculate score`))

(fn `Calculate score`
  ;[1 1 1] Calculate score by multiplying the recorded events by the score value
  (set `self.Score` (- (+ (* (`self.CarsReachedDest`) 5) (* (`self.PedsReachDest`) 5)) (+ (* (`self.Acidents`) 5) (* (`self.RoadRage`) 5)))))

(fn `UpdateCurrentSave`
  ;[1 1 1] Update Current Save
  (`/Game/Blueprints/SaveBlueprint/PlayerProfile.updateStats` (`self.Current`) (`self.Score`) (`self.Time`) (`self.CarsReachedDest`) (`self.PedsReachDest`) (`self.Acidents`) (`self.RoadRage`)))

(fn `UserConstructionScript`)