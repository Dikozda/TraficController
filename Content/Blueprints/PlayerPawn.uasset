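; Player pawn with an orthographic top-down camera that lets the player drag fire ants from nests onto cars to trigger road rage.
; Touching a nest spawns a blob that follows the finger; releasing destroys it and sphere-traces to max out nearby smart cars' rage.
; It also creates the HUD, handles camera-yaw-relative movement and clamped mouse-wheel zoom, and offers a timeline-driven random screen shake.
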(event `Shake`
  ;[1 1 1] Screen shake
  (bind (_direction _newtrack_0) (`Timeline|Screen shake falloff` :!via `PlayFromStart`)
    (:`Update`
      (`SceneComponent.K2_SetRelativeRotation` (`self.Camera`) (`KismetMathLibrary.MakeRotator` (* (* 20.0 _newtrack_0) (`KismetMathLibrary.RandomFloatInRange` -1.0 1.0)) -90.0) false false)
      (`SceneComponent.K2_SetRelativeLocation` (`self.Camera`) (`KismetMathLibrary.MakeVector` (* (* 50.0 _newtrack_0) (`KismetMathLibrary.RandomFloatInRange` -1.0 1.0)) (* (* 50.0 _newtrack_0) (`KismetMathLibrary.RandomFloatInRange` -1.0 1.0))) false false))))

(event `self.ReceiveBeginPlay`
  ;[1 1 1] Hud
  (`/Engine/EditorBlueprintResources/StandardMacros.IsValid` (`self.HUDRef`)
    (:`Is Valid`
      _)
    (:`Is Not Valid`
      (bind _returnvalue (`|CreateWidget` "/Game/Blueprints/UserInterface/Hud.Hud_C"))
      (bind _output_get (set `self.HUDRef` _returnvalue))))
  (`UserWidget.AddToViewport` _output_get 0))

(event `InputAxis|Move Forward`
  (params (AxisValue :type "Float (single-precision)"))
  (bind (_returnvalue_roll _returnvalue_pitch _returnvalue_yaw) (`KismetMathLibrary.BreakRotator` (`SceneComponent.K2_GetComponentRotation` (`self.Camera`))))
  ;[1 1 1] Movement Controls
  (`self.AddMovementInput` (`KismetMathLibrary.GetForwardVector` (`KismetMathLibrary.MakeRotator` 0.0 0.0 _returnvalue_yaw)) AxisValue))

(event `InputAxis|Move Right`
  (params (AxisValue :type "Float (single-precision)"))
  (bind (_returnvalue_roll _returnvalue_pitch _returnvalue_yaw) (`KismetMathLibrary.BreakRotator` (`SceneComponent.K2_GetComponentRotation` (`self.Camera`))))
  ;[1 1 1] Movement Controls
  (`self.AddMovementInput` (`KismetMathLibrary.GetRightVector` (`KismetMathLibrary.MakeRotator` 0.0 0.0 _returnvalue_yaw)) AxisValue))

(event `InputTouch`
  (params (Location :type "Vector Structure") (FingerIndex :type "ETouchIndex Enum"))
  (bind _hitresult (`PlayerController.GetHitResultUnderFingerByChannel` (`GameplayStatics.GetPlayerController` 0) FingerIndex "TraceTypeQuery1" true))
  ;[1 1 1] Input touch
  (:`Pressed`
    ;;[1 1 1] If a fire ant nest is clicked, spawn a fier ant
    (if (== (`GameplayStatics.GetObjectClass` (`.HitActor` (`GameplayStatics.BreakHitResult` _hitresult))) "/Game/Blueprints/DragAndDrop/BP_FireAntNest.BP_FireAntNest_C")
      (bind _returnvalue (`|SpawnActorFromClass` "/Game/Blueprints/DragAndDrop/FireAntBlob.FireAntBlob_C" (`KismetMathLibrary.MakeTransform` (`.Location` (`GameplayStatics.BreakHitResult` _hitresult))) "Undefined" "OverrideRootScale"))
      (set `self.FireAntBlob` _returnvalue)))
  (:`Released`
    ;;[1 1 1] When released execute fireant mayham
    (if (`KismetSystemLibrary.IsValid` (`self.FireAntBlob`))
      (`self.FireAntExplosion` 0 FingerIndex)))
  (:`Moved`
    ;;[1 1 1] Update location
    (if (`KismetSystemLibrary.IsValid` (`self.FireAntBlob`))
      (`self.K2_SetActorLocation` (`self.FireAntBlob`) (`KismetMathLibrary.MakeVector` (.x (`.TraceStart` (`GameplayStatics.BreakHitResult` _hitresult))) (.y (`.TraceStart` (`GameplayStatics.BreakHitResult` _hitresult))) 200.0) false false))))

(event `Key|MouseScrollDown`
  (params (Key :type "Key Structure" :default "AnyKey"))
  (bind _camera (`self.Camera`))
  ;[1 1 1] Zoom out
  (:`Pressed`
    (`CameraComponent.SetOrthoWidth` _camera (`KismetMathLibrary.FClamp` (+ (`CameraComponent.OrthoWidth` _camera) 100.0) 500.0 1000.0))))

(event `Key|MouseScrollUp`
  (params (Key :type "Key Structure" :default "AnyKey"))
  (bind _camera (`self.Camera`))
  ;[1 1 1] Zoom in
  (:`Pressed`
    (`CameraComponent.SetOrthoWidth` _camera (`KismetMathLibrary.FClamp` (- (`CameraComponent.OrthoWidth` _camera) 100.0) 500.0 1000.0))))

(fn `FireAntExplosion`
  (params (NewParam :type Byte) (FingerIndex :type "ETouchIndex Enum"))
  (bind _returnvalue (- (`self.K2_GetActorLocation` (`self.FireAntBlob`)) (0.0 0.0 50.0)))
  ;[1 1 1] Get all cars in a sphere around the fire ant blob and set their rage to 99999, effectivly forcing them to enter a road rage
  (bind _outhits (`KismetSystemLibrary.SphereTraceMulti` :`Start` _returnvalue :`End` _returnvalue :`Radius` 300.0 :`TraceChannel` "TraceTypeQuery1" :`DrawDebugType` "ForDuration"))
  (`self.K2_DestroyActor` (`self.FireAntBlob`))
  (for _array_element _outhits
    (if (== (`GameplayStatics.GetObjectClass` (`.HitActor` (`GameplayStatics.BreakHitResult` _array_element))) "/Game/Blueprints/Trafic/RoadTrafic/BP_SmartCar.BP_SmartCar_C")
      (bind _asbp_smart_car (cast `/Game/Blueprints/Trafic/RoadTrafic/BP_SmartCar` (`.HitActor` (`GameplayStatics.BreakHitResult` _array_element))))
      (set `/Game/Blueprints/Trafic/RoadTrafic/BP_SmartCar.Rage meter` 999999999999.0 _asbp_smart_car))))

(fn `UserConstructionScript`)