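; Train that follows a spline via its parent's Tick and asks the track to spawn another train as it nears the spline's end.
; A front bumper overlap with a smart car starts that car's crash despawn, enables physics on it and pauses the train's movement for a few seconds.
; The hit car then receives an impulse scaled by speed and mass at a point found by a forward line trace.
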(event `self.ReceiveTick`
  (params (DeltaSeconds :type "Float (single-precision)"))
  ;[1 1 1] IF can move is false, dont allow the train to move
  (if (`self.CanMove`)
    (`parent.ReceiveTick` DeltaSeconds)
    ;[1 1 1] check if the train has reached the end of the spline, and if so, call the train spline and tell it to spawn a new train
    (if (>= (`self.DistanceAlongSpline`) (- (`SplineComponent.GetSplineLength` (`/Game/Blueprints/Trafic/BP_Spline_Parent.Spline` (`self.CurrentSpline`))) 10.0))
      (bind _asbp_train_spline (cast `/Game/Blueprints/Trafic/Train/BP_TrainSpline` (`self.CurrentSpline`)))
      (`/Game/Blueprints/Trafic/Train/BP_TrainSpline.Spawn` _asbp_train_spline))))

(event `self.Front bumper.OnComponentBeginOverlap`
  (params (OverlappedComponent :type "PrimitiveComponent Object Reference") (OtherActor :type "Actor Object Reference") (OtherComp :type "PrimitiveComponent Object Reference") (OtherBodyIndex :type Integer) (bFromSweep :type Boolean) (SweepResult :type "HitResult Structure (by ref)"))
  ;[1 1 1] When the front bumper hits anouther actor, check if it is a car, if so, call the smash car function, if not, ignor it for now
  (if (== (`GameplayStatics.GetObjectClass` OtherActor) "/Game/Blueprints/Trafic/RoadTrafic/BP_SmartCar.BP_SmartCar_C")
    (`self.Smash Car` OtherActor)))

(event `MovementDelay`
  ;[1 1 1] When the movement delay is called, set can move to false, wait 5 seconds, then set can move to true
  (set `self.CanMove` false)
  (`KismetSystemLibrary.Delay` 5.0)
  (set `self.CanMove` true))

(fn `Smash Car`
  (params (`Car to smash` :type "Actor Object Reference"))
  (locals (NewVar_0 :type "Array of EObjectTypeQuery Enum") (CrashedCar :type "/Game/Blueprints/Trafic/RoadTrafic/BP_SmartCar Object Reference"))
  (bind _front_bumper (`self.Front bumper`))
  (bind _returnvalue (`SceneComponent.K2_GetComponentLocation` _front_bumper))
  ;[1 1 1] When the train hits a car headon, save the hit car as a local variable and call the crash despawn function, then simulate its physics and call the movement delay function in order to stop the trains movement for a small period of time the should allow the car to despawn befor it starts moveing again
  (bind _asbp_smart_car (cast `/Game/Blueprints/Trafic/RoadTrafic/BP_SmartCar` `Car to smash`))
  (bind _output_get (set `local.CrashedCar` _asbp_smart_car))
  (`/Game/Blueprints/Trafic/RoadTrafic/BP_SmartCar.Crash despawn` _output_get)
  (`PrimitiveComponent.SetSimulatePhysics` (`Character.CapsuleComponent` _output_get) true)
  (`self.MovementDelay`)
  ;[1 1 1] Do a line trace in front of the car to find where the car impacted
  (bind _outhit (`KismetSystemLibrary.LineTraceSingleForObjects` :`Start` _returnvalue :`End` (+ _returnvalue (* (`SceneComponent.GetForwardVector` _front_bumper) 100.0)) :`ObjectTypes` (`local.NewVar_0`) :`DrawDebugType` "ForOneFrame"))
  ;[1 1 1] Apply impulse at impact point, impulse strength is based on the force of the colision
  (`PrimitiveComponent.AddImpulseAtLocation` (`/Game/Blueprints/Trafic/RoadTrafic/BP_SmartCar.Box` (`local.CrashedCar`)) (* (`SceneComponent.GetForwardVector` (`self.Front bumper`)) (* (`self.CarSpeed`) (`self.Mass`))) (`.ImpactPoint` (`GameplayStatics.BreakHitResult` _outhit)) "None"))

(fn `UserConstructionScript`
  (`parent.UserConstructionScript`))