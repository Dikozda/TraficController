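; BP_TrainBarrier is a 2D train barrier that the player toggles by touch.
; On play it stops its Paper flipbook and holds a single frame as the initial state.
; Each touch on the flipbook alternates through a FlipFlop, switching collision on two boxes off or back on while jumping to the matching frame.
; The flipbook serves as a two-state sprite rather than a playing animation.
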(event `self.ReceiveBeginPlay`
  (bind _paperflipbook (`self.PaperFlipbook`))
  (`PaperFlipbookComponent.Stop` _paperflipbook)
  (`PaperFlipbookComponent.SetPlaybackPositionInFrames` _paperflipbook 1 false))

(event `self.PaperFlipbook.OnInputTouchBegin`
  (params (FingerIndex :type "ETouchIndex Enum" :default "Touch1") (TouchedComponent :type "PrimitiveComponent Object Reference"))
  (bind _paperflipbook (`self.PaperFlipbook`))
  (bind _box (`self.Box`))
  (bind _box1 (`self.Box1`))
  (`/Engine/EditorBlueprintResources/StandardMacros.FlipFlop`
    (:`A`
      (`PrimitiveComponent.SetCollisionEnabled` _box "NoCollision")
      (`PrimitiveComponent.SetCollisionEnabled` _box1 "NoCollision")
      (`PaperFlipbookComponent.SetPlaybackPositionInFrames` _paperflipbook 2 false))
    (:`B`
      (`PrimitiveComponent.SetCollisionEnabled` _box "QueryAndPhysics")
      (`PrimitiveComponent.SetCollisionEnabled` _box1 "QueryAndPhysics")
      (`PaperFlipbookComponent.SetPlaybackPositionInFrames` _paperflipbook 1 false))))

(fn `UserConstructionScript`)