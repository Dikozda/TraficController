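; Pedestrian crossing waypoint in the traffic system that the player opens and closes by touching its Left or Right arrow.
; Either touch toggles CanCross and keeps both arrow flipbooks in sync, with the frame showing the crossing state.
; Opening releases every walker in WaitingWalkers and clears the array.
; CrashDelay forces the crossing closed and calls CrashWait, which briefly ignores touches through the Delay flag.
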(event `CrashWait`
  ;[1 1 1] When called set delay to true, wait four seconds and then set delay to false
  (set `self.Delay` true)
  (`KismetSystemLibrary.Delay` 4.0)
  (set `self.Delay` false))

(event `self.ReceiveBeginPlay`
  (bind _left (`self.Left`))
  (bind _right (`self.Right`))
  ;[1 1 1] Event Begin Play
  (`parent.ReceiveBeginPlay`)
  ;;[1 1 1] Stop both flip books and then set them to frame 1, this is so they can be changed later and so they are both in sync
  (`|ExecutionSequence`
    (:`then_0`
      (`PaperFlipbookComponent.Stop` _right)
      (`PaperFlipbookComponent.SetPlaybackPositionInFrames` _right 1 false))
    (:`then_1`
      (`PaperFlipbookComponent.Stop` _left)
      (`PaperFlipbookComponent.SetPlaybackPositionInFrames` _left 1 false))))

(event `self.Left.OnInputTouchBegin`
  (params (FingerIndex :type "ETouchIndex Enum" :default "Touch1") (TouchedComponent :type "PrimitiveComponent Object Reference"))
  ;[1 1 1] When arrows have been touched, swtich the flip books between frames and change the can cross varible, if delay is true, nothing will happen
  (if (`self.Delay`) :!label _label
    _
    (elif (`self.CanCross`)
      (set `self.CanCross` false)
      (`PaperFlipbookComponent.SetPlaybackPositionInFrames` (`self.Left`) 1 false)
      (`PaperFlipbookComponent.SetPlaybackPositionInFrames` (`self.Right`) 1 false)
      (else
        (set `self.CanCross` true)
        (`PaperFlipbookComponent.SetPlaybackPositionInFrames` (`self.Left`) 2 false)
        (`PaperFlipbookComponent.SetPlaybackPositionInFrames` (`self.Right`) 2 false)
        ;[1 1 1] for each walker, set waiting to false in order to get them moving again, then clear the waiting walkers array
        (for _array_element (`self.WaitingWalkers`)
          (set `/Game/Blueprints/Trafic/WalkingPeople/Walker.Waiting` false _array_element))
        (`KismetArrayLibrary.Array_Clear` (`self.WaitingWalkers`))))))

(event `self.Right.OnInputTouchBegin`
  (params (FingerIndex :type "ETouchIndex Enum" :default "Touch1") (TouchedComponent :type "PrimitiveComponent Object Reference"))
  ;[1 1 1] When arrows have been touched, swtich the flip books between frames and change the can cross varible, if delay is true, nothing will happen
  (goto _label))

(fn `CrashDelay`
  ;[1 1 1] When called set can cross to false so no pedestrians wil try to cross when there is a crash and set the flipbooks to frame 1 to show that the cossing is closed, then call crash wait, crash wait is external since it uses a delay
  (set `self.CanCross` false)
  (`PaperFlipbookComponent.SetPlaybackPositionInFrames` (`self.Left`) 1 false)
  (`PaperFlipbookComponent.SetPlaybackPositionInFrames` (`self.Right`) 1 false)
  (`self.CrashWait`))

(fn `UserConstructionScript`
  (`parent.UserConstructionScript`))