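; Entrance waypoint for the walking-people traffic system that spawns pedestrians at its own transform at random intervals.
; Tick runs through a half-second Delay, then rolls a random integer from zero to a countdown and spawns a Walker on zero.
; Each miss lowers the countdown to raise the odds, and a spawn resets it to its default.
; Spawned walkers receive this waypoint as both start and current waypoint.
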(event `self.ReceiveBeginPlay`)

(event `self.ReceiveTick`
  (params (DeltaSeconds :type "Float (single-precision)"))
  ;[1 1 1] Spawn a walker after a random interval of time
  (`KismetSystemLibrary.Delay` 0.5)
  (if (== (`KismetMathLibrary.RandomIntegerInRange` 0 (`self.Random Int`)) 0)
    (`|SpawnActorFromClass` "/Game/Blueprints/Trafic/WalkingPeople/Walker.Walker_C" (`self.GetTransform`) "Undefined" "OverrideRootScale" null self self)
    (set `self.Random Int` (`self.Random Int Deafault`))
    (else
      (`/Engine/EditorBlueprintResources/StandardMacros.DecrementInt` (`self.Random Int`)))))

(fn `UserConstructionScript`
  (`parent.UserConstructionScript`))