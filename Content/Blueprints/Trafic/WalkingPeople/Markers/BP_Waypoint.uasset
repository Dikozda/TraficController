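; BP_Waypoint is a marker for walking-people traffic that discovers and stores its neighboring markers.
; CheckForMarkers casts debug-drawn line traces radially around the vertical axis, spaced by spoke count or a CustomAngle divisor.
; Hit waypoint, exit and crossing markers fill the Waypoints array; entrances are excluded.
; It rebuilds links on BeginPlay, and its construction script refreshes every BP_Waypoint to keep links current when one moves.
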(event `self.ReceiveBeginPlay`
  (`self.Check for markers`))

(event `self.ReceiveTick`
  (params (DeltaSeconds :type "Float (single-precision)")))

(fn `Check for markers`
  (bind _returnvalue (`self.K2_GetActorLocation`))
  (bind _spokes (`self.Spokes`))
  ;[1 1 1] Clear the array in order to reset the function
  (`KismetArrayLibrary.Array_Clear` (`self.Waypoints`))
  ;[1 1 1] Do a loop for each spoke, and use the current index to decide which direction to do the line trace
  (for _index (range 1 (+ _spokes 1))
    ;[1 1 1] Check line trace results to see if they are any of the waypoints, excluding the entrance, and add them to the waypoints array
    (bind _outhit (`KismetSystemLibrary.LineTraceSingle` :`Start` _returnvalue :`End` (+ _returnvalue (`KismetMathLibrary.RotateAngleAxis` (* (`self.GetActorForwardVector`) 1000) (* _index (/ 360.0 (`KismetMathLibrary.Conv_IntToDouble` (select `bool` (`self.UseSpokes`) :`false` (`self.CustomAngle`) :`true` _spokes)))) (0.0 0.0 1.0))) :`TraceChannel` "TraceTypeQuery3" :`DrawDebugType` "ForDuration" :`DrawTime` 2.0))
    (bind (_bblockinghit _binitialoverlap _time _location _impactpoint _normal _impactnormal _physmat _hitactor) (`GameplayStatics.BreakHitResult` _outhit))
    (bind _returnvalue_2 (`GameplayStatics.GetObjectClass` _hitactor))
    (if (or (== _returnvalue_2 "BP_Waypoint_C") (== _returnvalue_2 "/Game/Blueprints/Trafic/WalkingPeople/Markers/BP_Waypoint_Exit.BP_Waypoint_Exit_C") (== _returnvalue_2 "/Game/Blueprints/Trafic/WalkingPeople/Markers/BP_Waypoint_Crossing.BP_Waypoint_Crossing_C"))
      (bind _asbp_marker (cast `/Game/Blueprints/Trafic/WalkingPeople/Markers/BP_Marker` _hitactor))
      (`KismetArrayLibrary.Array_Add` (`self.Waypoints`) _asbp_marker))))

(fn `UserConstructionScript`
  ;[1 1 1] this is done in order to keep all the waypoints up to date when is moved
  (bind _outactors (`GameplayStatics.GetAllActorsOfClass` "BP_Waypoint_C"))
  (for _array_element _outactors
    (`self.Check for markers` _array_element)))