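; Base traffic vehicle that drives along the spline of its owning BP_Spline_Parent and destroys itself at the end.
; Each tick, unless crashed, it places itself at its current spline distance, then advances that distance by speed, axis value and delta time.
; A front bumper overlap zeroes the speed to stop the car, and the overlap ending restores a fixed driving speed.
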(event `self.ReceiveBeginPlay`
  ;[1 1 1] Gets a refernce of all Spline actors and stores them for later use
  (bind _asbp_spline_parent (cast `/Game/Blueprints/Trafic/BP_Spline_Parent` (`self.GetOwner`)))
  (set `self.CurrentSpline` _asbp_spline_parent))

(event `self.ReceiveTick`
  (params (DeltaSeconds :type "Float (single-precision)"))
  ;[1 1 1] If the vehicale has crashed, we dont want it to keep moving
  (if (not (`self.Crash`))
    ;[1 1 1] These two functions control the movement of this actor
    (`self.UpdateLocationAndRotation`)
    (`self.AddMovement`)))

(event `self.Front bumper.OnComponentBeginOverlap`
  (params (OverlappedComponent :type "PrimitiveComponent Object Reference") (OtherActor :type "Actor Object Reference") (OtherComp :type "PrimitiveComponent Object Reference") (OtherBodyIndex :type Integer) (bFromSweep :type Boolean) (SweepResult :type "HitResult Structure (by ref)"))
  ;[1 1 1] When the actor is blocked from the front, the seed is set to 0, which basicly stops the actor from moving.
  (set `self.Front blocked` true)
  (set `self.CarSpeed` 0.0))

(event `self.Front bumper.OnComponentEndOverlap`
  (params (OverlappedComponent :type "PrimitiveComponent Object Reference") (OtherActor :type "Actor Object Reference") (OtherComp :type "PrimitiveComponent Object Reference") (OtherBodyIndex :type Integer))
  ;[1 1 1] When the front of the car is clear, set the speed to a vlaue higher then 0 in order to get it moving again
  (set `self.Front blocked` false)
  (set `self.CarSpeed` 80.0))

(fn `AddMovement`
  (bind _returnvalue (* (`self.CarSpeed`) (`self.AxisValue`)))
  ;[1 1 1] This calculates the cars accleration and updates the distance along spline variable, when used with the update location and rotation function simulates movement
  (set `self.CarAccleration` _returnvalue)
  (set `self.DistanceAlongSpline` (+ (`self.DistanceAlongSpline`) (* _returnvalue (`GameplayStatics.GetWorldDeltaSeconds`)))))

(fn `UpdateLocationAndRotation`
  (locals (Delay :type "Float (double-precision)"))
  (if (>= (`self.DistanceAlongSpline`) (`SplineComponent.GetSplineLength` (`/Game/Blueprints/Trafic/BP_Spline_Parent.Spline` (`self.CurrentSpline`))))
    ;[1 1 1] When the actor of reached the end of the spline, destroy the actor
    (`self.K2_DestroyActor`)
    (else
      ;[1 1 1] Set Location and rotation on spline based on the distance along spline varible, which gets updated every tick
      (`self.K2_SetActorLocationAndRotation` (`SplineComponent.GetLocationAtDistanceAlongSpline` (`/Game/Blueprints/Trafic/BP_Spline_Parent.Spline` (`self.CurrentSpline`)) (`self.DistanceAlongSpline`) "World") (`SplineComponent.GetRotationAtDistanceAlongSpline` (`/Game/Blueprints/Trafic/BP_Spline_Parent.Spline` (`self.CurrentSpline`)) (`self.DistanceAlongSpline`) "World")))))

(fn `UserConstructionScript`)