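; BP_SmartSpline is a road traffic spline that, when flagged as a spawner, spawns vehicles at its start.
; It spawns one on BeginPlay, then uses a Delay in Tick to roll a random chance every half second, narrowing the range after each miss.
; A winning roll box-traces at the actor's location: a hit widens the range, while a clear trace spawns and resets it.
; Spawned BP_SmartCars receive this spline as CurrentSpline.
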(event `self.ReceiveBeginPlay`
  ;[1 1 1] Spawn the first Vehicel to get everything rolling
  (if (`self.IsSpawn`)
    (`self.Spawn Vehical`)))

(event `self.ReceiveTick`
  (params (DeltaSeconds :type "Float (single-precision)"))
  (bind _returnvalue (`self.K2_GetActorLocation`))
  ;[1 1 1] If this spline is set to spawn, check every half second if a randon interger in a range is equal to 0, if not, reduce the max range, wich will make it more likely to return true every time it checks
  (if (`self.IsSpawn`)
    (`KismetSystemLibrary.Delay` 0.5)
    (if (== (`KismetMathLibrary.RandomIntegerInRange` 0 (`self.Random Int`)) 0)
      ;[1 1 1] Do a box trace around the car spawn to see if there are any obsticals in the way of the spawn, if so, increase the max range of the random int, else spawn the vehicale and set the random int back to defualt
      (bind (_outhit _returnvalue_2) (`KismetSystemLibrary.BoxTraceSingle` :`Start` _returnvalue :`End` _returnvalue :`HalfSize` (45.0 25.0 5.0) :`Orientation` (`self.K2_GetActorRotation`) :`TraceChannel` "TraceTypeQuery1" :`DrawDebugType` "ForDuration"))
      (if _returnvalue_2
        (set `self.Random Int` (+ (`self.Random Int`) 2))
        (else
          (`self.Spawn Vehical`)
          (set `self.Random Int` (`self.Random Int Defualt`))))
      (else
        (`/Engine/EditorBlueprintResources/StandardMacros.DecrementInt` (`self.Random Int`))))))

(fn `Spawn Vehical`
  (bind _spline (`self.Spline`))
  ;[1 1 1] Spawn a vehical at the start of the spline and set it's spline indexs to match this actors trafic spline interger
  (bind _returnvalue (`|SpawnActorFromClass` (`self.SpawnType`) (`KismetMathLibrary.MakeTransform` (`SplineComponent.GetLocationAtDistanceAlongSpline` _spline 0.0 "World") (`SplineComponent.GetRotationAtDistanceAlongSpline` _spline 0.0 "World")) "Undefined" "OverrideRootScale" self))
  (bind _asbp_smart_car (cast `/Game/Blueprints/Trafic/RoadTrafic/BP_SmartCar` _returnvalue))
  (set `/Game/Blueprints/Trafic/RoadTrafic/BP_SmartCar.CurrentSpline` self _asbp_smart_car))

(fn `UserConstructionScript`)