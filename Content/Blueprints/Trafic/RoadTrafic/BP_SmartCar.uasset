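; AI traffic car that follows BP_SmartSpline roads, picks a random connected spline at each end and scores on reaching a final one.
; Randomized stats drive acceleration and a rage meter that fills while stopped, triggering full-speed road rage that ignores blockages.
; Front bumper overlaps either queue behind rear bumpers or crash into cars and walkers with physics impulses.
; Car crashes stall nearby cars and crossings, then despawn both vehicles.
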(event `self.ReceiveBeginPlay`
  (bind _paperflipbook (`self.PaperFlipbook`))
  ;[1 1 1] Begin Play
  ;;[1 1 1] Gets a refernce of the first spline this car is on
  (bind _asbp_smart_spline (cast `/Game/Blueprints/Trafic/RoadTrafic/BP_SmartSpline` (`self.GetOwner`)))
  (set `self.CurrentSpline` _asbp_smart_spline)
  ;;[1 1 1] Stop flipbook so it will allow custion positions
  (`PaperFlipbookComponent.Stop` _paperflipbook)
  (`PaperFlipbookComponent.SetPlaybackPositionInFrames` _paperflipbook 1 false))

(event `self.ReceiveTick`
  (params (DeltaSeconds :type "Float (single-precision)"))
  (bind _returnvalue (- (`self.Rage meter`) (`GameplayStatics.GetWorldDeltaSeconds`)))
  (bind _returnvalue_2 (+ (`self.CarSpeed`) (* (`self.CarAccleration`) (`GameplayStatics.GetWorldDeltaSeconds`))))
  ;[1 1 1] Event Tick
  (`|ExecutionSequence`
    (:`then_0`
      ;;[1 1 1] Movement
      (if (`self.Front blocked`)
        ;;;[1 1 1] Add the rage when not moving
        (set `self.Rage meter` (+ (`self.Rage meter`) (`GameplayStatics.GetWorldDeltaSeconds`)) :!label _label)
        (else
          ;;;[1 1 1] If the vehicale has crashed, we dont want it to keep moving
          (if (`self.Crash`)
            (goto _label)
            (elif (`self.CrashWait`)
              (goto _label)
              (else
                ;;;[1 1 1] These two functions control the movement of this actor
                (`self.UpdateLocationAndRotation`)
                (`self.AddMovement`)
                ;;;[1 1 1] Take rage away when moving
                (if (not (<= _returnvalue 0.0))
                  (set `self.Rage meter` _returnvalue))))))))
    (:`then_1`
      ;;[1 1 1] When rage is full, activate road rage
      (if (`self.RoadRage`)
        _
        (elif (>= (`self.Rage meter`) (`self.MaxRage`))
          (`self.ActivateRoadRage`)
          (`/Game/Blueprints/TraficControler.Add to score` (`self.GameModeRef`) 0 0 0 1))))
    (:`then_2`
      (if (not (`self.RoadRage`))
        ;;[1 1 1] Randomly decrease cars speed to 20
        (if (>= (`KismetMathLibrary.RandomFloatInRange` 0.0 100.0) 0.02)
          ;;[1 1 1] Increace speed of car when not waiting
          (if (not (or (> _returnvalue_2 (`self.MaxSpeed`)) (< _returnvalue_2 50.0)))
            (set `self.CarSpeed` _returnvalue_2))
          (else
            (`KismetSystemLibrary.Delay` 1.0)
            (set `self.CarSpeed` 50.0)))))))

(event `self.Front bumper.OnComponentEndOverlap`
  (params (OverlappedComponent :type "PrimitiveComponent Object Reference") (OtherActor :type "Actor Object Reference") (OtherComp :type "PrimitiveComponent Object Reference") (OtherBodyIndex :type Integer))
  ;[1 1 1] When the front of the car is clear, set the speed to a vlaue higher then 0 in order to get it moving again
  (if (`self.CrashWait`)
    _
    (elif (not (`self.RoadRage`))
      (set `self.Front blocked` false)
      (set `self.CarSpeed` 80.0))))

(event `Crash wait`
  ;[1 1 1] This to make the car stop moving and wait for the crash to disapear
  (set `self.CrashWait` true)
  (`KismetSystemLibrary.Delay` 5.0)
  (set `self.CrashWait` false))

(event `Crash despawn`
  ;[1 1 1] This is so the car despawns when there is a crash
  (`ActorComponent.Deactivate` (`self.PSleft`))
  (`ActorComponent.Deactivate` (`self.PSright`))
  (`PaperFlipbookComponent.SetPlaybackPositionInFrames` (`self.PaperFlipbook`) 2 false)
  (set `self.CarSpeed` 0.0)
  (`KismetSystemLibrary.Delay` 4.5)
  (`self.K2_DestroyActor`))

(event `self.Front bumper.OnComponentBeginOverlap`
  (params (OverlappedComponent :type "PrimitiveComponent Object Reference") (OtherActor :type "Actor Object Reference") (OtherComp :type "PrimitiveComponent Object Reference") (OtherBodyIndex :type Integer) (bFromSweep :type Boolean) (SweepResult :type "HitResult Structure (by ref)"))
  ;[1 1 1] If there was a crash, call the activate crash function, if not, set front to blocked and set speed to 0
  (if (`self.Crash`)
    _
    (elif (not (`self.CrashWait`))
      (bind (_crash _other_actor_return _iswalker) (`self.Crash Check` OtherComp OtherActor))
      (if _crash
        (`self.Activate Crash` _other_actor_return _iswalker)
        (elif (not (`self.RoadRage`))
          (set `self.Front blocked` true)
          (set `self.CarSpeed` 0.0))))))

(fn `Activate Crash`
  (params (OtherActor :type "Actor Object Reference") (Iswalker :type Boolean))
  (locals (CrashedCar :type "/Game/Blueprints/Trafic/RoadTrafic/BP_SmartCar Object Reference") (Walker :type "/Game/Blueprints/Trafic/WalkingPeople/Walker Object Reference"))
  (bind _returnvalue (`self.K2_GetActorLocation`))
  (bind _front_bumper (`self.Front bumper`))
  (bind _returnvalue_2 (`SceneComponent.K2_GetComponentLocation` _front_bumper))
  ;[1 1 1] Add 1 to the acident count in the gamemode and then check if the other actor is a walker or not
  (`/Game/Blueprints/TraficControler.Add to score` (`self.GameModeRef`) 0 0 1 0)
  (if Iswalker
    ;[1 1 1] Store a refernce to the crashed walker for later use
    (bind _aswalker (cast `/Game/Blueprints/Trafic/WalkingPeople/Walker` OtherActor))
    (bind _output_get (set `local.Walker` _aswalker))
    ;[1 1 1] call the crash function for the walker and enable physics for it
    (`/Game/Blueprints/Trafic/WalkingPeople/Walker.Crash` _output_get)
    (`PrimitiveComponent.SetSimulatePhysics` (`/Game/Blueprints/Trafic/WalkingPeople/Walker.Sphere` _output_get) true)
    ;[1 1 1] Do a line trace in front of the car to find where the car impacted
    (bind _outhit (`KismetSystemLibrary.LineTraceSingleForObjects` :`Start` (`SceneComponent.K2_GetComponentLocation` (`self.Front bumper`)) :`End` (`self.K2_GetActorLocation` (`local.Walker`)) :`ObjectTypes` (`self.NewVar_0`) :`DrawDebugType` "ForOneFrame"))
    ;[1 1 1] Apply impulse at impact point, impulse strength is based on the force of the colision
    (`PrimitiveComponent.AddImpulseAtLocation` (`/Game/Blueprints/Trafic/WalkingPeople/Walker.Sphere` (`local.Walker`)) (* (`SceneComponent.GetForwardVector` (`self.Front bumper`)) (* (`self.CarSpeed`) 1500.0)) (`.ImpactPoint` (`GameplayStatics.BreakHitResult` _outhit)) "None")
    ;[1 1 1] Activate road rage for the current car
    (`self.ActivateRoadRage`)
    (else
      ;[1 1 1] Store Refernce of the other crashed car for later use
      (bind _asbp_smart_car (cast `/Game/Blueprints/Trafic/RoadTrafic/BP_SmartCar` OtherActor))
      (set `local.CrashedCar` _asbp_smart_car)
      ;[1 1 1] Do a multibox trace around the area where the crash happend, and check if each item is a car or a crossing, if its a car, call its crash wait function so the wait for the crash to clear up, else if it s a crossing, call its crossing delay function
      (bind _outhits (`KismetSystemLibrary.BoxTraceMulti` :`Start` _returnvalue :`End` _returnvalue :`HalfSize` (100.0 100.0 100.0) :`TraceChannel` "TraceTypeQuery1" :`DrawDebugType` "ForDuration"))
      (for _array_element _outhits
        (bind (_bblockinghit _binitialoverlap _time _location _impactpoint _normal _impactnormal _physmat _hitactor) (`GameplayStatics.BreakHitResult` _array_element))
        (bind _returnvalue_3 (`GameplayStatics.GetObjectClass` _hitactor))
        (if (== _returnvalue_3 "BP_SmartCar_C")
          (bind _asbp_smart_car_2 (cast `/Game/Blueprints/Trafic/RoadTrafic/BP_SmartCar` _hitactor))
          (`self.Crash wait` _asbp_smart_car_2)
          (elif (== _returnvalue_3 "/Game/Blueprints/Trafic/WalkingPeople/Markers/BP_Waypoint_Crossing.BP_Waypoint_Crossing_C")
            (bind _asbp_waypoint_crossing (cast `/Game/Blueprints/Trafic/WalkingPeople/Markers/BP_Waypoint_Crossing` _hitactor))
            (`/Game/Blueprints/Trafic/WalkingPeople/Markers/BP_Waypoint_Crossing.CrashDelay` _asbp_waypoint_crossing))))
      ;[1 1 1] Enable physics on both cars so impulse will work
      (`PrimitiveComponent.SetSimulatePhysics` (`Character.CapsuleComponent` (`local.CrashedCar`)) true)
      (`PrimitiveComponent.SetSimulatePhysics` (`self.CapsuleComponent`) true)
      ;[1 1 1] Do a line trace in front of the car to find where the car impacted
      (bind _outhit_2 (`KismetSystemLibrary.LineTraceSingleForObjects` :`Start` _returnvalue_2 :`End` (+ _returnvalue_2 (* (`SceneComponent.GetForwardVector` _front_bumper) 100.0)) :`ObjectTypes` (`self.NewVar_0`) :`DrawDebugType` "ForOneFrame"))
      (`ActorComponent.Activate` (`self.Crahs_PS`) true)
      ;[1 1 1] Apply impulse at impact point, impulse strength is based on the force of the colision
      (`PrimitiveComponent.AddImpulseAtLocation` (`/Game/Blueprints/Trafic/RoadTrafic/BP_SmartCar.Box` (`local.CrashedCar`)) (* (`SceneComponent.GetForwardVector` (`self.Front bumper`)) (* (`self.CarSpeed`) (`PrimitiveComponent.GetMass` (`self.CapsuleComponent`)))) (`.ImpactPoint` (`GameplayStatics.BreakHitResult` _outhit_2)) "None")
      (`|ExecutionSequence`
        (:`then_0`
          (set `self.Crash` true))
        (:`then_1`
          ;[1 1 1] Set both crashed cars to despawn
          (`self.Crash despawn` (`local.CrashedCar`))
          (`self.Crash despawn`)
          (bind _outactors (`GameplayStatics.GetAllActorsOfClass` "/Game/Blueprints/PlayerPawn.PlayerPawn_C"))
          (`/Game/Blueprints/PlayerPawn.Shake` (`|GetArrayItem` _outactors))
          (`ActorComponent.Activate` (`self.Crahs_PS`) true))))))

(fn `ActivateRoadRage`
  ;[1 1 1] When called, set road rage to true, set car speed to max speed, and set crsh wait and front blocked to false, this will make the car go at full speed and wait for no-one, most likely going to cause a car crash
  (set `self.RoadRage` true)
  (set `self.CarSpeed` (`self.MaxSpeed`))
  (set `self.CrashWait` false)
  (set `self.Front blocked` false)
  ;[1 1 1] Activate particles as visual indicator of rage
  (`ActorComponent.Activate` (`self.PSleft`) false)
  (`ActorComponent.Activate` (`self.PSright`) false))

(fn `AddMovement`
  ;[1 1 1] This calculates the cars accleration and updates the distance along spline variable, when used with the update location and rotation function simulates movement
  (set `self.DistanceAlongSpline` (+ (`self.DistanceAlongSpline`) (* (* (`self.CarSpeed`) (`self.AxisValue`)) (`GameplayStatics.GetWorldDeltaSeconds`)))))

(fn `Crash Check`
  (params (`Overlaped Component` :type "ActorComponent Object Reference") (`Other actor` :type "Actor Object Reference"))
  (returns (Crash :type Boolean) (`Other actor Return` :type "Actor Object Reference") (ISWalker :type Boolean))
  (bind _returnvalue (`GameplayStatics.GetObjectClass` `Other actor`))
  ;[1 1 1] Check if the other actor is ether a smart car, walker or other
  (if (== _returnvalue "BP_SmartCar_C")
    ;[1 1 1] Check to see if the front bumber colided with a rear bumber, if it did, set crash to false, if not, set crash to true.
    (bind _asbp_smart_car (cast `/Game/Blueprints/Trafic/RoadTrafic/BP_SmartCar` `Other actor`)
      (:`then`
        (if (!= (`/Game/Blueprints/Trafic/RoadTrafic/BP_SmartCar.Rear bumper` _asbp_smart_car) `Overlaped Component`)
          (return true `Other actor` false)
          (else
            _)))
      (:`CastFailed`
        _))
    (return false `Other actor` false)
    (elif (== _returnvalue "/Game/Blueprints/Trafic/WalkingPeople/Walker.Walker_C")
      (return true `Other actor` true)
      (else
        (return false `Other actor` false)))))

(fn `FindNewSpline`
  (locals (SplineArray :type "Array of Actor Object Reference"))
  (bind _returnvalue (`self.K2_GetActorLocation`))
  (bind _splinearray (`local.SplineArray`))
  ;[1 1 1] Clear the spline array in order to reset this function
  (`KismetArrayLibrary.Array_Clear` (`local.SplineArray`))
  ;[1 1 1] Do a multisphere trace in order to find any nearby splines
  (bind _outhits (`KismetSystemLibrary.SphereTraceMulti` :`Start` _returnvalue :`End` _returnvalue :`Radius` 10.0 :`TraceChannel` "TraceTypeQuery4" :`DrawDebugType` "ForDuration"))
  ;[1 1 1] Fore each actor that reacted to the sphere trace that used the spline colision channle, check to see if it is a spline by casting to smart spline and then add it to the spline array
  (for _array_element _outhits
    (bind (_bblockinghit _binitialoverlap _time _location _impactpoint _normal _impactnormal _physmat _hitactor) (`GameplayStatics.BreakHitResult` _array_element))
    (cast `/Game/Blueprints/Trafic/RoadTrafic/BP_SmartSpline` _hitactor)
    (`KismetArrayLibrary.Array_Add` (`local.SplineArray`) _hitactor))
  ;[1 1 1] Get a random spline from the spline array and set it as the current spline
  (bind _asbp_smart_spline (cast `/Game/Blueprints/Trafic/RoadTrafic/BP_SmartSpline` (`|GetArrayItem` _splinearray (`KismetMathLibrary.RandomIntegerInRange` 0 (`KismetArrayLibrary.Array_LastIndex` _splinearray)))))
  (bind _output_get (set `self.CurrentSpline` _asbp_smart_spline))
  ;[1 1 1] Check to see if the current spline is a turning spline, if so, check to see if it will be turning left or right and set the flipbook position acordingly, else set the flipbook position back to deafult
  (if (`/Game/Blueprints/Trafic/RoadTrafic/BP_SmartSpline.IsTurning` _output_get)
    (if (`/Game/Blueprints/Trafic/RoadTrafic/BP_SmartSpline.TurnRight` _output_get)
      (set `self.Turn Right` true)
      (`PaperFlipbookComponent.SetPlaybackPositionInFrames` (`self.PaperFlipbook`) 4 false)
      (else
        (set `self.Turn left` true)
        (`PaperFlipbookComponent.SetPlaybackPositionInFrames` (`self.PaperFlipbook`) 3 false)))
    (else
      (`PaperFlipbookComponent.SetPlaybackPositionInFrames` (`self.PaperFlipbook`) 1 false))))

(fn `UpdateLocationAndRotation`
  (locals (Delay :type "Float (double-precision)"))
  (if (>= (`self.DistanceAlongSpline`) (`SplineComponent.GetSplineLength` (`/Game/Blueprints/Trafic/RoadTrafic/BP_SmartSpline.Spline` (`self.CurrentSpline`))))
    ;[1 1 1] If the current spline if the end, get the gamemode ref and call the add to score function and then destroy self, else call the find new spline function and set distance along spline back to 0
    (if (`/Game/Blueprints/Trafic/RoadTrafic/BP_SmartSpline.IsEnd` (`self.CurrentSpline`))
      (`/Game/Blueprints/TraficControler.Add to score` (`self.GameModeRef`) 1 0 0 0)
      ;;[1 1 1] When the actor of reached the end of the spline, destroy the actor
      (`self.K2_DestroyActor`)
      (else
        (`self.FindNewSpline`)
        (set `self.DistanceAlongSpline` 0.0)))
    (else
      ;[1 1 1] Set Location and rotation on spline based on the distance along spline varible, which gets updated every tick
      (`self.K2_SetActorLocationAndRotation` (`SplineComponent.GetLocationAtDistanceAlongSpline` (`/Game/Blueprints/Trafic/RoadTrafic/BP_SmartSpline.Spline` (`self.CurrentSpline`)) (`self.DistanceAlongSpline`) "World") (`SplineComponent.GetRotationAtDistanceAlongSpline` (`/Game/Blueprints/Trafic/RoadTrafic/BP_SmartSpline.Spline` (`self.CurrentSpline`)) (`self.DistanceAlongSpline`) "World")))))

(fn `UserConstructionScript`
  ;[1 1 1] Get a Gamemode refernce and save it
  (bind _astrafic_controler (cast `/Game/Blueprints/TraficControler` (`GameplayStatics.GetGameMode`)))
  (set `self.GameModeRef` _astrafic_controler)
  ;[1 1 1] Random stats
  (set `self.MaxRage` (`KismetMathLibrary.RandomFloatInRange` 30.0 70.0))
  (set `self.MaxSpeed` (`KismetMathLibrary.RandomFloatInRange` 90.0 300.0))
  (set `self.CarAccleration` (`KismetMathLibrary.RandomFloatInRange` 5.0 50.0)))