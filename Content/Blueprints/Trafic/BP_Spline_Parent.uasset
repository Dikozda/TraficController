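; BP_Spline_Parent is a traffic lane actor that spawns vehicles at the start of its spline.
; It spawns one on BeginPlay, then on Tick, while active and SpawnEmpty is set, runs a delayed random roll whose odds rise after each miss.
; Vehicles leaving SpawnBox set SpawnEmpty.
; The construction script re-indexes all instances by array position, and spawned BP_Vehicle_Parent actors receive that index as SplineIndex.
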(event `self.ReceiveBeginPlay`
  ;[1 1 1] Spawn a vehicle at the start of the game to get everything rolling
  (`self.Spawn Vehical`))

(event `self.ReceiveTick`
  (params (DeltaSeconds :type "Float (single-precision)"))
  ;[1 1 1] This makes the spawn a bit more random in order to make the trafic a bit more spread out and randomly distributed
  (if (`self.SpawnActive`)
    (if (`self.Spawn empty`)
      (`KismetSystemLibrary.Delay` 0.5)
      (if (== (`KismetMathLibrary.RandomIntegerInRange` 0 (`self.Random Int`)) 0)
        (`self.Spawn Vehical`)
        (set `self.Random Int` (`self.Random Int Defualt`))
        (else
          (`/Engine/EditorBlueprintResources/StandardMacros.DecrementInt` (`self.Random Int`)))))))

(event `self.Spawn Box.OnComponentEndOverlap`
  (params (OverlappedComponent :type "PrimitiveComponent Object Reference") (OtherActor :type "Actor Object Reference") (OtherComp :type "PrimitiveComponent Object Reference") (OtherBodyIndex :type Integer))
  ;[1 1 1] When a vehical leaves the spawn box, set spawn empty to true
  (set `self.Spawn empty` true))

(fn `Spawn Vehical`
  (bind _spline (`self.Spline`))
  ;[1 1 1] Spawn a vehical at the start of the spline and set it's spline indexs to match this actors trafic spline interger
  (bind _returnvalue (`|SpawnActorFromClass` (`self.SpawnType`) (`KismetMathLibrary.MakeTransform` (`SplineComponent.GetLocationAtDistanceAlongSpline` _spline 0.0 "World") (`SplineComponent.GetRotationAtDistanceAlongSpline` _spline 0.0 "World")) "Undefined" "OverrideRootScale" self))
  (bind _asbp_vehicle_parent (cast `/Game/Blueprints/Trafic/BP_Vehicle_Parent` _returnvalue))
  (set `/Game/Blueprints/Trafic/BP_Vehicle_Parent.Spline Index` (`self.Trafic Spline`) _asbp_vehicle_parent))

(fn `Update index`
  (params (TraficPline :type "Array of /Game/Blueprints/Trafic/BP_Spline_Parent Object Reference"))
  ;[1 1 1] Find this actor in the all actors of class array and set trafic spline int to the indexs, this is so each trafic spline placed in the level will have its own int set by default
  (set `self.Trafic Spline` (`KismetArrayLibrary.Array_Find` TraficPline self)))

(fn `UserConstructionScript`
  ;[1 1 1] Setup the Trafic spline interger for all trafic spline actors in order to save me some hassel when i place a new trafic spline actor
  (bind _outactors (`GameplayStatics.GetAllActorsOfClass` "BP_Spline_Parent_C"))
  (for _array_element _outactors
    (`self.Update index` _array_element _outactors)))