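; PlayerProfile is a save-data Blueprint that holds a player's cumulative statistics for what appears to be a traffic game.
; It tracks score, time played, vehicles and pedestrians reaching their destinations, accidents and traffic delays.
; UpdateStats adds incoming values to the stored totals, and ClearStats resets every total to zero.
; Neither function writes to a save slot itself.
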(fn `ClearStats`
  ;[1 1 1] Set all varibles to 0 in order to "clear" the data
  (set `self.score` 0)
  (set `self.TimePlayed` 0.0)
  (set `self.VehiclesRechingDestination` 0)
  (set `self.PedestriansReachingDestination` 0)
  (set `self.Acidents` 0)
  (set `self.TraficDelays` 0))

(fn `updateStats`
  (params (Score :type Integer) (TimePlayed :type "Float (double-precision)") (VehiclesReachingDestination :type Integer) (PedestriansReachingDestination :type Integer) (Acidents :type Integer) (TraficDelays :type Integer))
  ;[1 1 1] Add value to saved varibles
  (set `self.score` (+ Score (`self.score`)))
  (set `self.TimePlayed` (+ TimePlayed (`self.TimePlayed`)))
  (set `self.VehiclesRechingDestination` (+ VehiclesReachingDestination (`self.VehiclesRechingDestination`)))
  (set `self.PedestriansReachingDestination` (+ PedestriansReachingDestination (`self.PedestriansReachingDestination`)))
  (set `self.Acidents` (+ Acidents (`self.Acidents`)))
  (set `self.TraficDelays` (+ TraficDelays (`self.TraficDelays`)))
  (return))