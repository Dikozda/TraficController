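; TraficSpline is a placeable traffic lane actor that spawns AI Vehicle pawns at the start of its spline.
; A vehicle spawns at BeginPlay and whenever a component leaves SpawnBox, unless CarArray holds nine or more entries.
; The construction script re-indexes every TraficSpline in the level by its array position, and each spawned vehicle receives that index as SplineIndex.
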(event `self.ReceiveBeginPlay`
  (`self.Spawn Vehical`))

(event `self.ReceiveTick`
  (params (DeltaSeconds :type "Float (single-precision)")))

(event `self.Spawn Box.OnComponentEndOverlap`
  (params (OverlappedComponent :type "PrimitiveComponent Object Reference") (OtherActor :type "Actor Object Reference") (OtherComp :type "PrimitiveComponent Object Reference") (OtherBodyIndex :type Integer))
  (`self.Spawn Vehical`))

(fn `Spawn Vehical`
  (bind _spline (`self.Spline`))
  (if (not (>= (`KismetArrayLibrary.Array_Length` (`self.Car Array`)) 9))
    (bind _returnvalue (`AIBlueprintHelperLibrary.SpawnAIFromClass` "/Game/Blueprints/Vehicle.Vehicle_C" null (`SplineComponent.GetLocationAtDistanceAlongSpline` _spline 0.0 "World") (`SplineComponent.GetRotationAtDistanceAlongSpline` _spline 0.0 "World")))
    (bind _asvehicle (cast `/Game/Blueprints/Vehicle` _returnvalue))
    (set `/Game/Blueprints/Vehicle.Spline Index` (`self.Trafic Spline`) _asvehicle)))

(fn `Update index`
  (params (TraficPline :type "Array of /Game/Blueprints/TraficSpline Object Reference"))
  ;[1 1 1] Find this actor in the all actors of class array and set trafic spline int to the indexs, this is so each trafic spline placed in the level will have its own int set by default
  (set `self.Trafic Spline` (`KismetArrayLibrary.Array_Find` TraficPline self)))

(fn `UserConstructionScript`
  (bind _outactors (`GameplayStatics.GetAllActorsOfClass` "TraficSpline_C"))
  (for _array_element _outactors
    (`self.Update index` _array_element _outactors)))