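; PlayerPawn is a player-controlled pawn with camera-relative movement and mouse-wheel zoom on an orthographic camera.
; The Move Forward and Move Right axes feed AddMovementInput along directions built from only the camera's world yaw, so camera pitch does not affect movement.
; Mouse-wheel presses step the camera's ortho width up or down within a clamped range.
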(event `InputAxis|Move Forward`
  (params (AxisValue :type "Float (single-precision)"))
  (bind (_returnvalue_roll _returnvalue_pitch _returnvalue_yaw) (`KismetMathLibrary.BreakRotator` (`SceneComponent.K2_GetComponentRotation` (`self.Camera`))))
  (`self.AddMovementInput` (`KismetMathLibrary.GetForwardVector` (`KismetMathLibrary.MakeRotator` 0.0 0.0 _returnvalue_yaw)) AxisValue))

(event `InputAxis|Move Right`
  (params (AxisValue :type "Float (single-precision)"))
  (bind (_returnvalue_roll _returnvalue_pitch _returnvalue_yaw) (`KismetMathLibrary.BreakRotator` (`SceneComponent.K2_GetComponentRotation` (`self.Camera`))))
  (`self.AddMovementInput` (`KismetMathLibrary.GetRightVector` (`KismetMathLibrary.MakeRotator` 0.0 0.0 _returnvalue_yaw)) AxisValue))

(event `Key|MouseScrollDown`
  (params (Key :type "Key Structure" :default "AnyKey"))
  (bind _camera (`self.Camera`))
  (:`Pressed`
    (`CameraComponent.SetOrthoWidth` _camera (`KismetMathLibrary.FClamp` (+ (`CameraComponent.OrthoWidth` _camera) 100.0) 500.0 2000.0))))

(event `Key|MouseScrollUp`
  (params (Key :type "Key Structure" :default "AnyKey"))
  (bind _camera (`self.Camera`))
  (:`Pressed`
    (`CameraComponent.SetOrthoWidth` _camera (`KismetMathLibrary.FClamp` (- (`CameraComponent.OrthoWidth` _camera) 100.0) 500.0 2000.0))))

(fn `UserConstructionScript`)