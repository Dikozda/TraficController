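; Touch-toggled traffic light actor that switches between stop and go states.
; On BeginPlay it stops its Paper2D flipbook on frame 1, using flipbook frames as static light states.
; Touching the flipbook drives a FlipFlop: go disables the Box collision and shows frame 2, stop restores collision and frame 1.
; Each switch also prints its state.
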(event `self.ReceiveBeginPlay`
  (bind _paperflipbook (`self.PaperFlipbook`))
  (`PaperFlipbookComponent.Stop` _paperflipbook)
  (`PaperFlipbookComponent.SetPlaybackPositionInFrames` _paperflipbook 1 false))

(event `self.PaperFlipbook.OnInputTouchBegin`
  (params (FingerIndex :type "ETouchIndex Enum" :default "Touch1") (TouchedComponent :type "PrimitiveComponent Object Reference"))
  (`/Engine/EditorBlueprintResources/StandardMacros.FlipFlop`
    (:`A`
      (`PrimitiveComponent.SetCollisionEnabled` (`self.Box`) "NoCollision")
      (`KismetSystemLibrary.PrintString` "go")
      (`PaperFlipbookComponent.SetPlaybackPositionInFrames` (`self.PaperFlipbook`) 2 false))
    (:`B`
      (`PrimitiveComponent.SetCollisionEnabled` (`self.Box`) "QueryAndPhysics")
      (`KismetSystemLibrary.PrintString` "stop")
      (`PaperFlipbookComponent.SetPlaybackPositionInFrames` (`self.PaperFlipbook`) 1 false))))

(fn `UserConstructionScript`)